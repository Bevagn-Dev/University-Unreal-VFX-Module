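; BP_Targets is a damageable target actor that explodes when its health runs out.
; Health starts at MaxHealth, and AnyDamage subtracts from it with clamping, calling Death at zero.
; Death destroys the static mesh, then requests an NS_Explosion Niagara effect attached to that same component, using actor world X/Y as a relative offset.
; The actor destroys itself after a short delay.
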(event `self.ReceiveBeginPlay`
  ;[1 1 1] Begin
  (set `self.Current Health` (`self.MaxHealth`)))

(event `self.ReceiveAnyDamage`
  (params (Damage :type "Float (single-precision)") (DamageType :type "DamageType Object Reference") (InstigatedBy :type "Controller Object Reference") (DamageCauser :type "Actor Object Reference"))
  ;[1 1 1] Health
  (bind _output_get (set `self.Current Health` (`KismetMathLibrary.FClamp` (- (`self.Current Health`) Damage) 0.0 (`self.MaxHealth`))))
  (if (<= _output_get 0.0)
    (`self.Death`)))

(event `Death`
  (bind (_returnvalue_x _returnvalue_y) (`KismetMathLibrary.BreakVector` (`self.K2_GetActorLocation`)))
  (bind _staticmesh (`self.StaticMesh`))
  ;[1 1 1] Death
  (`ActorComponent.K2_DestroyComponent` _staticmesh)
  (`NiagaraFunctionLibrary.SpawnSystemAttached` "/Game/VFX/LessonStuff/NS_Explosion.NS_Explosion" _staticmesh "None" (`KismetMathLibrary.MakeVector` _returnvalue_x _returnvalue_y 50.0) (struct) "KeepRelativeOffset")
  (`KismetSystemLibrary.Delay` 1.0)
  (`self.K2_DestroyActor`))

(fn `UserConstructionScript`)