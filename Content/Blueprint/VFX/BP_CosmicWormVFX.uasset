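; Cosmic worm VFX actor that delivers a delayed area hit with damage and a physical push.
; After a wind-up delay, VFXPlay briefly pulses a RadialForce and, at the same moment, damages actors found by a capsule overlap.
; The capsule follows the actor's X and Y but sits at a fixed world height.
; The actor destroys itself shortly after the pulse only if flagged IsSpawned.
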(event `self.ReceiveBeginPlay`
  (`parent.ReceiveBeginPlay`))

(event `self.VFXPlay`
  (bind (_returnvalue_x _returnvalue_y) (`KismetMathLibrary.BreakVector` (`self.K2_GetActorLocation`)))
  (bind _radialforce (`self.RadialForce`))
  (`KismetSystemLibrary.Delay` 1.3)
  (`|ExecutionSequence`
    (:`then_0`
      (`ActorComponent.Activate` _radialforce true)
      (`KismetSystemLibrary.Delay` 0.2)
      (`ActorComponent.Deactivate` _radialforce)
      (`KismetSystemLibrary.Delay` 0.5)
      (if (`self.IsSpawned`)
        (`self.K2_DestroyActor`)))
    (:`then_1`
      (bind _outactors (`KismetSystemLibrary.CapsuleOverlapActors` (`KismetMathLibrary.MakeVector` _returnvalue_x _returnvalue_y 160.0) 90.0 200.0 (`self.Object Types`)))
      (for _array_element _outactors
        (`GameplayStatics.ApplyDamage` _array_element 50.0)))))

(fn `UserConstructionScript`
  (`parent.UserConstructionScript`))