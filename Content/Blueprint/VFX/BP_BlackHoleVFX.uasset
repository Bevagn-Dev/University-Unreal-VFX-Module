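; Black hole VFX actor that pairs the effect with a timed radial force and area damage.
; The radial force starts inactive; on VFXPlay it activates after a delay, alongside a single radial damage hit with falloff at the actor's XY and a fixed world height.
; After a short window the force deactivates, and the actor destroys itself if IsSpawned is set.
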(event `self.ReceiveBeginPlay`
  (`parent.ReceiveBeginPlay`)
  (`ActorComponent.Deactivate` (`self.RadialForce`)))

(event `self.VFXPlay`
  (bind (_returnvalue_x _returnvalue_y) (`KismetMathLibrary.BreakVector` (`self.K2_GetActorLocation`)))
  (bind _radialforce (`self.RadialForce`))
  (`KismetSystemLibrary.Delay` 1.66)
  (`ActorComponent.Activate` _radialforce true)
  (`GameplayStatics.ApplyRadialDamageWithFalloff` :`BaseDamage` 25.0 :`MinimumDamage` 10.0 :`Origin` (`KismetMathLibrary.MakeVector` _returnvalue_x _returnvalue_y 100.0) :`DamageInnerRadius` 250.0 :`DamageOuterRadius` 350.0 :`DamageFalloff` 1.0 :`DamageCauser` null :`InstigatedByController` null)
  (`KismetSystemLibrary.Delay` 1.0)
  (`ActorComponent.Deactivate` _radialforce)
  (if (`self.IsSpawned`)
    (`self.K2_DestroyActor`)))

(fn `UserConstructionScript`
  (`parent.UserConstructionScript`))