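; Meteor VFX actor that turns particle data from its Niagara system into damage and physics impulses.
; When flagged as spawned, it registers itself as the Niagara export callback handler on BeginPlay and destroys itself after a short delay.
; For each exported particle position, it sphere-overlaps actors, damages each hit actor, and moves and fires a shared RadialForce component, which starts deactivated.
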(event `self.ReceiveBeginPlay`
  (`ActorComponent.Deactivate` (`self.RadialForce`))
  (if (`self.IsSpawned`)
    (`NiagaraComponent.SetNiagaraVariableObject` (`self.Niagara`) "BPCallbackHandler" self)
    (`KismetSystemLibrary.Delay` 1.5)
    (`self.K2_DestroyActor`)))

(event `self.ReceiveParticleData`
  (params (Data :type "Array of BasicParticleData Structure (by ref)") (NiagaraSystem :type "NiagaraSystem Object Reference") (SimulationPositionOffset :type "Vector Structure (by ref)"))
  (bind _radialforce (`self.RadialForce`))
  (for _array_element Data
    (bind _position (break `BasicParticleData` _array_element))
    (bind _outactors (`KismetSystemLibrary.SphereOverlapActors` _position 100.0 (`self.Object Types`)))
    (for _array_element_2 _outactors
      (`GameplayStatics.ApplyDamage` _array_element_2 25.0)
      (`ActorComponent.Activate` _radialforce true)
      (`SceneComponent.K2_SetWorldLocation` _radialforce _position false false)
      (`RadialForceComponent.FireImpulse` _radialforce))))

(fn `UserConstructionScript`)