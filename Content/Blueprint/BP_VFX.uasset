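; BP_VFX is an actor that spawns a Niagara system at its own location when play begins.
; The UseActorRotation flag decides whether the system takes the actor's rotation or a zero rotation.
; After spawning, it calls VFXPlay, an event left empty in this Blueprint.
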(event `self.ReceiveBeginPlay`
  (`self.SpawnVFX`))

(event `SpawnVFX`
  (if (`self.UseActorRotation`)
    (set `self.NSRotation` (`self.K2_GetActorRotation`))
    (else
      (set `self.NSRotation` (struct))))
  (`NiagaraFunctionLibrary.SpawnSystemAtLocation` (`self.NS System`) (`self.K2_GetActorLocation`) (`self.NSRotation`))
  (`self.VFXPlay`))

(event `VFXPlay`)

(fn `UserConstructionScript`)